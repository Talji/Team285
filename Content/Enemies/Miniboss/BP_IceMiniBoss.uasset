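; BP_IceMiniBoss is an ice miniboss enemy that patrols between two points and chases the player on sight.
; While it cannot see the player, Tick sends it back and forth between two hardcoded world locations, flipping ReachedSide on each successful move.
; Pawn Sensing starts a chase toward BP_Player, and a half-second retriggerable delay clears CanSeeEnemy to resume patrol once sightings stop.
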(event `self.ReceiveBeginPlay`)

(event `self.ReceiveTick`
  (params (DeltaSeconds :type "Float (single-precision)"))
  (set `CharacterMovementComponent.MaxWalkSpeed` 100.0 (`self.CharacterMovement`))
  (if (not (`self.CanSeeEnemy?`))
    (if (`self.ReachedSide?`)
      (`|AIMoveTo` self (2637.0 3138.0 0.0) null
        (:`OnSuccess`
          (set `self.ReachedSide?` false)))
      (else
        (`|AIMoveTo` self (505.0 3122.0 0.0) null
          (:`OnSuccess`
            (set `self.ReachedSide?` true)))))))

(event `self.PawnSensing.OnSeePawn`
  (params (Pawn :type "Pawn Object Reference"))
  (set `CharacterMovementComponent.MaxWalkSpeed` 100.0 (`self.CharacterMovement`))
  (bind _asbp_player (cast `/Game/ThirdPerson/Blueprints/BP_Player` Pawn))
  (`|ExecutionSequence`
    (:`then_0`
      (set `self.CanSeeEnemy?` true)
      (`|AIMoveTo` self (0.0 0.0 0.0) _asbp_player))
    (:`then_1`
      (`KismetSystemLibrary.RetriggerableDelay` 0.5)
      (set `self.CanSeeEnemy?` false))))

(fn `UserConstructionScript`)