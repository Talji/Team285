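; Ranged enemy Blueprint that wanders, approaches a seen player and fires projectiles at close range.
; Tick drives delayed random wandering while no player is seen, with self-destruction after a delay if overlapping the player.
; PawnSensing sightings trigger either a chase or a stop and projectile spawn, by distance.
; A retriggerable delay clears the sight flag when sightings stop; Health is initialised but otherwise unused here.
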(event `self.ReceiveBeginPlay`
  (set `self.Health` 10.0))

(event `self.ReceiveTick`
  (params (DeltaSeconds :type "Float (single-precision)"))
  (if (not (`self.CanSeeEnemy?`))
    (`KismetSystemLibrary.Delay` (`KismetMathLibrary.RandomFloatInRange` 2.0 4.0))
    (`|AIMoveTo` self (`NavigationSystemV1.K2_GetRandomReachablePointInRadius` (`self.K2_GetActorLocation`) 500.0 null null) null
      (:`then`
        (if (`self.IsOverlappingActor` (`GameplayStatics.GetPlayerCharacter` 0))
          (`KismetSystemLibrary.Delay` 2.0)
          (`self.K2_DestroyActor`))))))

(event `self.PawnSensing.OnSeePawn`
  (params (Pawn :type "Pawn Object Reference"))
  (bind _asbp_player (cast `/Game/ThirdPerson/Blueprints/BP_Player` Pawn))
  (`|ExecutionSequence`
    (:`then_0`
      (set `self.CanSeeEnemy?` true)
      (if (> (`self.GetDistanceTo` (`GameplayStatics.GetPlayerCharacter` 0)) 500.0)
        (`|AIMoveTo` self (0.0 0.0 0.0) _asbp_player)
        (else
          (`NavMovementComponent.StopActiveMovement` (`self.CharacterMovement`))
          (`|SpawnActorFromClass` "/Game/Enemies/BP_EnemyProjectile.BP_EnemyProjectile_C" (`SceneComponent.K2_GetComponentToWorld` (`self.EnemyProjectileSpawner`)) "Undefined" "OverrideRootScale" null self)
          (`KismetSystemLibrary.Delay` 0.2))))
    (:`then_1`
      (`KismetSystemLibrary.RetriggerableDelay` 0.5)
      (set `self.CanSeeEnemy?` false))))

(fn `UserConstructionScript`)